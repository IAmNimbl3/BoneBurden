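; Wallrun component for BP_FirstPersonCharacter, providing start, stop, surface validation and wall-jump vector helpers.
; CheckWallrunnable requires a side-facing wall, enough forward speed, falling state and floor clearance.
; StartWallrun plane-constrains movement to the wall normal, zeroes vertical velocity, lowers gravity and starts height-hold and falloff timers; StopWallrun resets these.
; LaunchLogicCalc builds a launch vector from the wall normal, current speed and added height.
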(event `self.ReceiveBeginPlay`
  (bind _asbp_first_person_character (cast `/Game/Blueprints/Player/BP_FirstPersonCharacter` (`self.GetOwner`)))
  (bind _output_get (set `self.Owner` _asbp_first_person_character))
  (set `self.CharacterMovement` (`Character.CharacterMovement` _output_get)))

(event `OnHeightTimerFinish`
  (set `self.bCanMantainHeight` false)
  (bind _returnvalue (`KismetSystemLibrary.K2_SetTimerDelegate` (`|CreateDelegate` :!event `onFallEnd`) 2.0))
  (set `self.falloffWallrunTimer` _returnvalue))

(event `OnFallEnd`
  (`self.StopWallrun`))

(fn `CheckWallrunnable`
  (params (Hit :type "HitResult Structure"))
  (returns (Hit1 :type "HitResult Structure") (ReturnValue :type Boolean))
  (bind (_floorresult_bblockinghit _floorresult_bwalkablefloor _floorresult_blinetrace _floorresult_floordist) (break `FindFloorResult` (`CharacterMovementComponent.K2_FindFloor` (`self.CharacterMovement`) (`Actor.K2_GetActorLocation` (`self.Owner`)))))
  (return Hit (and (> (`KismetMathLibrary.Abs` (`KismetMathLibrary.Dot_VectorVector` (`.Normal` (`GameplayStatics.BreakHitResult` Hit)) (`Actor.GetActorRightVector` (`self.Owner`)))) 0.8) (> (`self.GetVelocityForward`) 500.0) (`NavMovementInterface.IsFalling` (`self.CharacterMovement`)) (> _floorresult_floordist 42.0))))

(fn `GetVelocityForward`
  (returns (ReturnValue :type String))
  (bind _owner (`self.Owner`))
  (return (`KismetStringLibrary.Conv_DoubleToString` (`KismetMathLibrary.VSize` (`KismetMathLibrary.Conv_DoubleToVector` (`KismetMathLibrary.Dot_VectorVector` (`Actor.GetVelocity` _owner) (`Actor.GetActorForwardVector` _owner)))))))

(fn `LaunchLogicCalc`
  (params (Factor :type "Float (double-precision)") (`Height Gained` :type "Float (double-precision)"))
  (returns (ReturnValue :type "Vector Structure"))
  (return (+ (* (`MovementComponent.GetPlaneConstraintNormal` (`self.CharacterMovement`)) (* (`KismetMathLibrary.VSize` (`Actor.GetVelocity` (`self.Owner`))) Factor)) (`KismetMathLibrary.MakeVector` 0.0 0.0 `Height Gained`))))

(fn `StartWallrun`
  (params (Normal :type "Vector Structure"))
  (bind _charactermovement (`self.CharacterMovement`))
  (bind _charactermovement_2 (`self.CharacterMovement`))
  (bind (_returnvalue_x _returnvalue_y _returnvalue_z) (`KismetMathLibrary.BreakVector` (`Actor.K2_GetActorLocation` (`self.Owner`))))
  (bind (_velocity_x _velocity_y) (`KismetMathLibrary.BreakVector` (`MovementComponent.Velocity` _charactermovement_2)))
  (`KismetSystemLibrary.K2_ClearAndInvalidateTimerHandle` (`self.MantainHeightTimer`))
  (`KismetSystemLibrary.K2_ClearAndInvalidateTimerHandle` (`self.FalloffWallrunTimer`))
  ; Stored height to use in eventgraph
  (set `self.StoredHeight` _returnvalue_z)
  (if (and (`NavMovementInterface.IsFalling` _charactermovement) (not (`self.bIsWallrunning`)))
    ; Constraint to movement + obtaining wall normal
    (`MovementComponent.SetPlaneConstraintEnabled` _charactermovement true)
    (`MovementComponent.SetPlaneConstraintNormal` _charactermovement Normal)
    (set `self.bIsWallrunning` true)
    (set `self.bCanMantainHeight` true)
    (set `self.FallSpeed` 0.0)
    (bind _returnvalue (`KismetSystemLibrary.K2_SetTimerDelegate` (`|CreateDelegate` :!event `onHeightTimerFinish`) 2.0))
    (set `self.MantainHeightTimer` _returnvalue)
    ; Wallrunning handler
    (set `CharacterMovementComponent.GravityScale` 0.25 (`self.CharacterMovement`))
    (bind _returnvalue_2 (`KismetSystemLibrary.K2_SetTimerDelegate` (`|CreateDelegate` :!event `stopWallrun`) 4.0))
    (set `self.FalloffWallrunTimer` _returnvalue_2)
    (set `MovementComponent.Velocity` (`KismetMathLibrary.MakeVector` _velocity_x _velocity_y) _charactermovement_2)))

(fn `StopWallrun`
  (`KismetSystemLibrary.K2_ClearAndInvalidateTimerHandle` (`self.mantainHeightTimer`))
  (`KismetSystemLibrary.K2_ClearAndInvalidateTimerHandle` (`self.falloffWallrunTimer`))
  (`MovementComponent.SetPlaneConstraintEnabled` (`self.CharacterMovement`) false)
  (set `self.bIsWallrunning` false)
  (set `self.fallSpeed` 0.0)
  (set `CharacterMovementComponent.GravityScale` 1.0 (`self.CharacterMovement`)))