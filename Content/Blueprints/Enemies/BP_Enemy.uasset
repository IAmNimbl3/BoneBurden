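; BP_Enemy is a melee enemy character that punches when the player pawn is in range and is destroyed by any damage it takes.
; An overlap volume toggles CanAttack, and Tick triggers Hit, which plays the punch montage with movement disabled until shortly after it completes.
; HitState toggles the hit collider, which damages each BPI_Damageable actor once per punch, skipping other BPI_Enemy actors.
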(event `self.ReceiveAnyDamage`
  (params (Damage :type "Float (single-precision)") (DamageType :type "DamageType Object Reference") (InstigatedBy :type "Controller Object Reference") (DamageCauser :type "Actor Object Reference"))
  (`self.K2_DestroyActor`))

(event `self.Can Hit Collision.OnComponentBeginOverlap`
  (params (OverlappedComponent :type "PrimitiveComponent Object Reference") (OtherActor :type "Actor Object Reference") (OtherComp :type "PrimitiveComponent Object Reference") (OtherBodyIndex :type Integer) (bFromSweep :type Boolean) (SweepResult :type "HitResult Structure (by ref)"))
  (if (== OtherActor (`GameplayStatics.GetPlayerPawn` 0))
    (set `self.bCanAttack` true)))

(event `self.Can Hit Collision.OnComponentEndOverlap`
  (params (OverlappedComponent :type "PrimitiveComponent Object Reference") (OtherActor :type "Actor Object Reference") (OtherComp :type "PrimitiveComponent Object Reference") (OtherBodyIndex :type Integer))
  (if (== (`GameplayStatics.GetPlayerPawn` 0) OtherActor)
    (set `self.bCanAttack` false)))

(event `Hit`
  (if (not (`self.bAttacking`))
    (`KismetArrayLibrary.Array_Clear` (`self.HittedActors`))
    (set `self.bAttacking` true)
    (`self.MovementState` false)
    (`|PlayMontage` (`self.Mesh`) "/Game/Characters/Demon/Animations/AM_Punch.AM_Punch"
      (:`OnCompleted`
        (`KismetSystemLibrary.Delay` 0.2)
        (`self.MovementState` true)
        (set `self.bAttacking` false)))))

(event `/Game/Blueprints/Enemies/BPI_Enemy.HitState`
  (params (CanHit :type Boolean))
  (bind _hit_collision (`self.Hit Collision`))
  (if CanHit
    (`PrimitiveComponent.SetCollisionEnabled` _hit_collision "QueryAndPhysics")
    (else
      (`PrimitiveComponent.SetCollisionEnabled` _hit_collision "NoCollision"))))

(event `self.Hit Collision.OnComponentBeginOverlap`
  (params (OverlappedComponent :type "PrimitiveComponent Object Reference") (OtherActor :type "Actor Object Reference") (OtherComp :type "PrimitiveComponent Object Reference") (OtherBodyIndex :type Integer) (bFromSweep :type Boolean) (SweepResult :type "HitResult Structure (by ref)"))
  (if (and (not (`KismetArrayLibrary.Array_Contains` (`self.HittedActors`) OtherActor)) (and (not (`KismetSystemLibrary.DoesImplementInterface` OtherActor "/Game/Blueprints/Enemies/BPI_Enemy.BPI_Enemy_C")) (`KismetSystemLibrary.DoesImplementInterface` OtherActor "/Game/Blueprints/BPI_Damageable.BPI_Damageable_C")))
    (`GameplayStatics.ApplyDamage` OtherActor 10.0 null null "/Script/Engine.DamageType")
    (`KismetArrayLibrary.Array_AddUnique` (`self.HittedActors`) OtherActor)))

(event `MovementState`
  (params (CanMove :type Boolean))
  (bind _charactermovement (`self.CharacterMovement`))
  (if CanMove
    (`CharacterMovementComponent.SetMovementMode` _charactermovement "MOVE_Walking" 0)
    (else
      (`CharacterMovementComponent.SetMovementMode` _charactermovement "MOVE_None" 0))))

(event `self.ReceiveTick`
  (params (DeltaSeconds :type "Float (single-precision)"))
  (if (`self.bCanAttack`)
    (`self.Hit`)))

(fn `UserConstructionScript`)