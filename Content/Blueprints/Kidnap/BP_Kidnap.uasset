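; Trigger actor that plays a kidnap cutscene with a spinning LordDemon when the first-person character enters its Box.
; On overlap it disables player movement, blends the view to itself, then runs a Timeline that drives LordDemon's yaw.
; Late in the spin the actor itself, not the player, teleports once to TargetLocation.
; Afterwards, delayed blends pass the view to AuxCamera, then back to the player as walking is restored.
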(event `self.Box.OnComponentBeginOverlap`
  (params (OverlappedComponent :type "PrimitiveComponent Object Reference") (OtherActor :type "Actor Object Reference") (OtherComp :type "PrimitiveComponent Object Reference") (OtherBodyIndex :type Integer) (bFromSweep :type Boolean) (SweepResult :type "HitResult Structure (by ref)"))
  (bind _returnvalue (`GameplayStatics.GetPlayerController` 0))
  (bind _asbp_first_person_character (cast `/Game/Blueprints/Player/BP_FirstPersonCharacter` OtherActor))
  (bind _output_get (set `self.Player` _asbp_first_person_character))
  (bind _output_get_2 (set `self.Character Movement` (`Character.CharacterMovement` _output_get)))
  (`CharacterMovementComponent.SetMovementMode` _output_get_2 "MOVE_None" 0)
  (`PlayerController.SetViewTargetWithBlend` (`GameplayStatics.GetPlayerController` 0) self 0.3 "VTBlend_Linear" 0.0 false)
  (`KismetSystemLibrary.Delay` 2.0)
  (bind (_direction _rotation) (`Timeline|Timeline` :!via `PlayFromStart`)
    (:`Update`
      (`SceneComponent.K2_SetRelativeRotation` (`self.Lord Demon`) (`KismetMathLibrary.MakeRotator` 0.0 0.0 _rotation) false false)
      (if (and (> _rotation 900.0) (not (`self.bHasTeleported`)))
        (`self.K2_SetActorLocation` (`self.TargetLocation`) false true)
        (set `self.bHasTeleported` true)))
    (:`Finished`
      (`KismetSystemLibrary.Delay` 2.5)
      (`PlayerController.SetViewTargetWithBlend` _returnvalue (`self.AuxCamera`) 5.0 "VTBlend_Linear" 0.0 false)
      (`KismetSystemLibrary.Delay` 5.0)
      (`CharacterMovementComponent.SetMovementMode` (`self.Character Movement`) "MOVE_Walking" 0)
      (`PlayerController.SetViewTargetWithBlend` _returnvalue (`self.Player`) 1.0 "VTBlend_Linear" 0.0 false))))

(fn `UserConstructionScript`)